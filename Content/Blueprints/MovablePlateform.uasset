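; MovablePlateform is a moving platform that oscillates smoothly back and forth between its Start and End components.
; Tick accumulates time and feeds it through a sine helper, remapped to a 0–1 range and scaled in frequency by Speed.
; PlateformePosition linearly interpolates between the two components' relative locations with that value, and the Cylinder is moved there each frame without sweeping.
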(event EventTick
  (params (DeltaSeconds :type Float%20%28single-precision%29))
  (bind _output_get (Variables|Default|SetTime (+ DeltaSeconds (Variables|Default|GetTime))))
  (bind _sin (CallFunction|SinCustom _output_get (Variables|Default|GetSpeed) 0.5 0.5 0.0))
  (bind _returnvalue (CallFunction|PlateformePosition _sin))
  (Transformation|SetRelativeLocation (Variables|Default|GetCylinder) _returnvalue false false))

(fn ConstructionScript)

(fn SinCustom
  (params (Angle :type Float%20%28double-precision%29) (Speed :type Float%20%28double-precision%29) (Amplitude :type Float%20%28double-precision%29) (Offset :type Float%20%28double-precision%29) (Phase :type Float%20%28double-precision%29))
  (return (+ (* (Math|Trig|Sin(Radians) (+ (* Angle Speed) Phase)) Amplitude) Offset)))

(fn PlateformePosition
  (params (offset :type Float%20%28double-precision%29))
  (bind _start (Variables|Default|GetStart))
  (bind _returnvalue (Transformation|GetRelativeTransform _start))
  (return (+ (* offset (- (.location (Transformation|GetRelativeTransform (Variables|Default|GetEnd))) (.location _returnvalue))) (.location _returnvalue))))