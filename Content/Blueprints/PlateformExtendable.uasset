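; Extendable platform that stretches along its X scale when ExtendPlateform is called.
; ExtendPlateform resets CurrentSize to 1, then AnimeExtend grows it using delta seconds and Speed and applies it to the Scene component's world scale, keeping Y and Z.
; A short Delay loops back into AnimeExtend until ValueExtend is reached, animating the stretch without Tick or a Timeline.
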(event Custom|ExtendPlateform
  (Variables|Default|SetCurrentSize 1.0)
  (CallFunction|AnimeExtend))

(event Custom|AnimeExtend
  (bind _scene (Variables|Default|GetScene))
  (bind _returnvalue (Transformation|GetWorldScale _scene))
  (bind _output_get (Variables|Default|SetCurrentSize (+ (* (stale EventTick DeltaSeconds) (Variables|Default|GetSpeed)) (+ (stale EventTick DeltaSeconds) (Variables|Default|GetCurrentSize)))))
  (Transformation|SetWorldScale3D _scene (Math|Vector|MakeVector _output_get (.y _returnvalue) (.z _returnvalue)))
  (if (< _output_get (Variables|Default|GetValueExtend))
    (Utilities|FlowControl|Delay 0.001)
    (CallFunction|AnimeExtend)))

(event EventBeginPlay)

(event EventTick
  (params (DeltaSeconds :type Float%20%28single-precision%29)))

(fn ConstructionScript)