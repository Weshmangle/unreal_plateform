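; Coin pickup actor that bobs vertically until collected, then plays a destroy sequence.
; Each tick, AnimeCoin offsets the location along local Z by a sine of accumulated time, seeded randomly at BeginPlay to vary phase between coins.
; CoinIsPickUp_Event disables sphere collision, plays a 2D explosion sound and starts DestroySequency.
; The DestroyCoin Sequencer event then destroys the actor.
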(event Custom|CoinIsPickUp_Event
  ;[1 1 1] Anime Pickup
  (Collision|SetCollisionEnabled (Variables|Default|GetSphere) "NoCollision")
  (Audio|PlaySound2D "/Game/Audio/Explosion_Cue.Explosion_Cue" 1.0 1.0 0.0 0 0)
  (Class|ActorSequenceComponent|PlaySequence (Variables|Default|GetDestroySequency)))

(event EventBeginPlay
  ;[1 1 1] Random Vertical Position Begin Play
  (Variables|Default|Settime (Math|Random|RandomFloat)))

(event EventTick
  (params (DeltaSeconds :type Float%20%28single-precision%29))
  ;[1 1 1] Animate Position
  (CallFunction|AnimeCoin DeltaSeconds))

(event Custom|DestroyCoin
  (params (Coin0 :type Actor%20Object%20Reference))
  (Actor|DestroyActor))

(fn ConstructionScript)

(fn AnimeCoin
  (params (deltaTime :type Float%20%28double-precision%29))
  (bind _output_get (Variables|Default|Settime (+ deltaTime (Variables|Default|Gettime))))
  (Transformation|SetActorTransform (Math|Conversions|ToTransform(Vector) (Math|Transform|TransformLocation (Transformation|GetActorTransform) (Math|Vector|MakeVector 0.0 0.0 (* (Math|Trig|Sin(Radians) (* _output_get 2.5)) 0.5))))))